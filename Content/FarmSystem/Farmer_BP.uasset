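; Farmer actor for the farm system that lets the player open and close a Farmer HUD while standing near it.
; Box overlap shows or hides a text prompt and enables or disables input on the actor.
; T toggles the menu through an IsOpen flag, creating FarmerHUD with the actor's UnitID and showing the mouse cursor.
; Closing hides the cursor and removes all widgets, not just this HUD.
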(event OnComponentBeginOverlap(Box)
  (params (OverlappedComponent :type Primitive%20Component%20Object%20Reference) (OtherActor :type Actor%20Object%20Reference) (OtherComp :type Primitive%20Component%20Object%20Reference) (OtherBodyIndex :type Integer) (bFromSweep :type Boolean) (SweepResult :type Hit%20Result%20Structure%20%28by%20ref%29))
  (Rendering|SetVisibility (Variables|Default|GetTextRender) true false)
  (Input|EnableInput (Game|GetPlayerController 0)))

(event OnComponentEndOverlap(Box)
  (params (OverlappedComponent :type Primitive%20Component%20Object%20Reference) (OtherActor :type Actor%20Object%20Reference) (OtherComp :type Primitive%20Component%20Object%20Reference) (OtherBodyIndex :type Integer))
  (Rendering|SetVisibility (Variables|Default|GetTextRender) false false)
  (Input|DisableInput (Game|GetPlayerController 0)))

(event EventBeginPlay)

(event Collision|EventActorBeginOverlap
  (params (OtherActor :type Actor%20Object%20Reference)))

(event EventTick
  (params (DeltaSeconds :type Float%20%28single-precision%29)))

(event Input|KeyboardEvents|T
  (params (Key :type Key%20Structure))
  (bind _returnvalue (Game|GetPlayerController 0))
  (:Pressed
    (if (Variables|Default|GetIsOpen)
      (Viewport|RemoveAllWidgets)
      (Variables|Default|SetIsOpen false)
      (Variables|/Script/Engine.PlayerController|SetbShowMouseCursor _returnvalue false)
      (else
        (bind _returnvalue_2 (UserInterface|CreateWidget "/Game/FarmSystem/New_UI/Farmer/FarmerHUD.FarmerHUD_C" 0 (Variables|Default|GetUnitID)))
        (UserInterface|Viewport|AddtoViewport _returnvalue_2 0)
        (Variables|Default|SetIsOpen true)
        (Variables|/Script/Engine.PlayerController|SetbShowMouseCursor _returnvalue true)))))

(fn ConstructionScript)