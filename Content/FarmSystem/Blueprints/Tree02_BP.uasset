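; Tree02_BP is a farm system Blueprint that scatters tree static meshes around the actor.
; Its construction script adds NumOfTrees mesh components, each at a random X and Y offset within configurable min and max ranges, with flat Z, no rotation and unit scale.
; A random stream drives the placement, so the layout is repeatable for a given seed.
; The event graph holds no active logic.
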(event EventBeginPlay)

(event Collision|EventActorBeginOverlap
  (params (OtherActor :type Actor%20Object%20Reference)))

(event EventTick
  (params (DeltaSeconds :type Float%20%28single-precision%29)))

(fn ConstructionScript
  (bind _stream (Variables|Default|GetStream))
  (for _index (range 1 (Variables|Default|GetNumOfTrees))
    (AddComponent|AddStaticMeshComponent false (Math|Transform|MakeTransform (Math|Vector|MakeVector (Math|Random|RandomFloatinRangefromStream (Variables|Default|GetMinValue_X) (Variables|Default|GetMaxValue_X) _stream) (Math|Random|RandomFloatinRangefromStream (Variables|Default|GetMinValue_Y) (Variables|Default|GetMaxValue_Y) _stream) 0.0)))))