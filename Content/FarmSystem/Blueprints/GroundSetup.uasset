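; GroundSetup is a farm-system Blueprint that lays out a rectangular grid of static mesh ground tiles.
; Its construction script runs nested X and Y loops, adding one mesh component per cell, spaced by GroundSize.
; Each component's relative transform includes the actor's world location, and the one-based indices start the grid one tile away from that point.
; The event graph holds only disabled placeholder events, with no runtime logic.
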(event EventBeginPlay)

(event Collision|EventActorBeginOverlap
  (params (OtherActor :type Actor%20Object%20Reference)))

(event EventTick
  (params (DeltaSeconds :type Float%20%28single-precision%29)))

(fn ConstructionScript
  (bind _groundsize (Variables|Default|GetGroundSize))
  (for _index (range 1 (Variables|Default|GetNumberOfGround_X))
    (for _index_2 (range 1 (Variables|Default|GetNumberOfGround_Y))
      (AddComponent|AddStaticMeshComponent false (Math|Transform|MakeTransform (+ (Transformation|GetActorLocation) (Math|Vector|MakeVector (Math|Conversions|ToFloat(Integer) (* _index _groundsize)) (Math|Conversions|ToFloat(Integer) (* _index_2 _groundsize)) 0.0)))))))