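; Farm field actor that tiles a ground mesh grid and mirrors its plot's state from a web database.
; BeginPlay fetches fields, matches FarmNo, labels availability and spawns a Farmer_BP on occupied plots.
; Tick re-requests the unit's data every frame, and each response adds plant-state meshes across the grid without removing earlier ones.
; Box overlap enables input so G toggles the FarmPlanHUD, which opens only for empty plots.
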(event OnComponentBeginOverlap(Box)
  (params (OverlappedComponent :type Primitive%20Component%20Object%20Reference) (OtherActor :type Actor%20Object%20Reference) (OtherComp :type Primitive%20Component%20Object%20Reference) (OtherBodyIndex :type Integer) (bFromSweep :type Boolean) (SweepResult :type Hit%20Result%20Structure%20%28by%20ref%29))
  (Variables|Default|SetIsInRange true)
  (Input|EnableInput (Game|GetPlayerController 0)))

(event OnComponentEndOverlap(Box)
  (params (OverlappedComponent :type Primitive%20Component%20Object%20Reference) (OtherActor :type Actor%20Object%20Reference) (OtherComp :type Primitive%20Component%20Object%20Reference) (OtherBodyIndex :type Integer))
  (Variables|Default|SetIsInRange false)
  (Development|PrintString "Bye")
  (Input|DisableInput (Game|GetPlayerController 0)))

(event Custom|Complete
  (params (Request :type Va%20Rest%20Request%20JSON%20Object%20Reference))
  (bind _returnvalue (Transformation|GetActorTransform))
  (bind _textrender (Variables|Default|GetTextRender))
  (bind _location (Math|Transform|BreakTransform _returnvalue))
  (bind (_x _y _z) (Math|Vector|BreakVector _location))
  (bind _json_return (CallFunction|GetDecodeJson Request (stale EventBeginPlay _return_json)))
  (for _array_element (Class|VaRestJsonObject|GetArrayField _json_return "Field")
    (bind _returnvalue_2 (Class|VaRestJsonValue|AsObject _array_element))
    (if (== (Variables|Default|GetFarmNo) (Math|Conversions|ToInteger(Byte) (Class|VaRestJsonObject|GetStringField _returnvalue_2 "no")))
      (Variables|Default|SetUnitID (Math|Conversions|ToInteger(Byte) (Class|VaRestJsonObject|GetStringField _returnvalue_2 "Unit_id")))
      (if (== (Math|Conversions|ToInteger(Byte) (Class|VaRestJsonObject|GetStringField _returnvalue_2 "isEmpty")) 0)
        (Variables|Default|SetisEmpty false)
        (Variables|Default|SetEmptyText "Unavailable")
        (Rendering|Components|TextRender|SetTextRenderColor _textrender (Variables|Default|GetColorRed))
        (else
          (Variables|Default|SetisEmpty true)
          (Variables|Default|SetEmptyText "Available")
          (Rendering|Components|TextRender|SetTextRenderColor _textrender (Variables|Default|GetColorGreen))))
      (Rendering|Components|TextRender|SetText _textrender (Utilities|Text|ToText(String) (Utilities|String|Append "FieldNo : " (Class|VaRestJsonObject|GetStringField _returnvalue_2 "no") "<br>Status : " (Variables|Default|GetEmptyText))))
      ;[1 1 1] Spawn Farmer
      (if (not (Variables|Default|GetisEmpty))
        (Game|SpawnActorfromClass "/Game/FarmSystem/Farmer_BP.Farmer_BP_C" (Math|Transform|MakeTransform (Math|Vector|MakeVector (- _x 5e+02) (- _y 3.5e+02) _z) "0,-90.000000, 0" "0.500000,0.500000,0.500000") "AdjustIfPossibleButAlwaysSpawn" 0 (Variables|Default|GetUnitID) 0)))))

(event Custom|Failure
  (params (Request :type Va%20Rest%20Request%20JSON%20Object%20Reference)))

(event Custom|ShowMesh
  (params (PlantState :type Integer))
  (bind _numberofground_x (Variables|Default|GetNumberOfGround_X))
  (bind _numberofground_y (Variables|Default|GetNumberOfGround_Y))
  (bind _groundsize (Variables|Default|GetGroundSize))
  (bind _groundsize_2 (Variables|Default|GetGroundSize))
  (for _index (range 1 _numberofground_x)
    (for _index_2 (range 1 _numberofground_y)
      (switch int PlantState
        (:0
          (AddComponent|AddStaticMeshComponent false (Math|Transform|MakeTransform (+ "-50.000000,-50.000000, 0" (Math|Vector|MakeVector (- (* _index _groundsize) (/ (* _numberofground_x _groundsize_2) 2.0)) (- (* _index_2 _groundsize) (/ (* _numberofground_y _groundsize_2) 2.0)) 0.0)))))
        (:1
          (AddComponent|AddStaticMeshComponent false (Math|Transform|MakeTransform (+ "-50.000000,-50.000000, 0" (Math|Vector|MakeVector (- (* _index _groundsize) (/ (* _numberofground_x _groundsize_2) 2.0)) (- (* _index_2 _groundsize) (/ (* _numberofground_y _groundsize_2) 2.0)) 0.0)))))
        (:2
          (AddComponent|AddStaticMeshComponent false (Math|Transform|MakeTransform (+ "-50.000000,-50.000000, 0" (Math|Vector|MakeVector (- (* _index _groundsize) (/ (* _numberofground_x _groundsize_2) 2.0)) (- (* _index_2 _groundsize) (/ (* _numberofground_y _groundsize_2) 2.0)) 0.0)))))
        (:3
          (AddComponent|AddStaticMeshComponent false (Math|Transform|MakeTransform (+ "-50.000000,-50.000000, 0" (Math|Vector|MakeVector (- (* _index _groundsize) (/ (* _numberofground_x _groundsize_2) 2.0)) (- (* _index_2 _groundsize) (/ (* _numberofground_y _groundsize_2) 2.0)) 0.0)))))
        (:4
          (AddComponent|AddStaticMeshComponent false (Math|Transform|MakeTransform (+ "-50.000000,-50.000000, 0" (Math|Vector|MakeVector (- (* _index _groundsize) (/ (* _numberofground_x _groundsize_2) 2.0)) (- (* _index_2 _groundsize) (/ (* _numberofground_y _groundsize_2) 2.0)) 0.0)))))))))

(event Custom|UnitComplete
  (params (Request :type Va%20Rest%20Request%20JSON%20Object%20Reference))
  (Development|PrintString "Complete")
  (bind _json_return (CallFunction|GetDecodeJson Request (stale EventTick _jsonreturn)))
  (for _array_element (Class|VaRestJsonObject|GetArrayField _json_return "Unit4Field")
    (bind _returnvalue (Class|VaRestJsonValue|AsObject _array_element))
    (Development|PrintString (Utilities|String|ToString(Integer) (Class|VaRestJsonObject|GetIntegerField _returnvalue "Unit_State")))
    (CallFunction|ShowMesh (Class|VaRestJsonObject|GetIntegerField _returnvalue "Unit_State"))))

(event Custom|UnitFail
  (params (Request :type Va%20Rest%20Request%20JSON%20Object%20Reference))
  (Development|PrintString "Fail"))

(event EventTick
  (params (DeltaSeconds :type Float%20%28single-precision%29))
  (bind _jsonreturn (CallFunction|GetUnitforField (delegate Custom|UnitComplete) (delegate Custom|UnitFail) (Variables|Default|GetUnitID))))

(event EventBeginPlay
  (bind _return_json (CallFunction|GetJsonfromDB "http://thebackyardfarm.fun/farm/getField.php?cid=1" (delegate Custom|Complete) (delegate Custom|Failure))))

(event Input|KeyboardEvents|G
  (params (Key :type Key%20Structure))
  (:Pressed
    (if (Variables|Default|GetIsShowFarmPlan)
      (Viewport|RemoveAllWidgets)
      (Variables|/Script/Engine.PlayerController|SetbShowMouseCursor (Game|GetPlayerController 0) false)
      (Variables|Default|SetIsShowFarmPlan false)
      (elif (Variables|Default|GetisEmpty)
        (bind _returnvalue (UserInterface|CreateWidget "/Game/FarmSystem/New_UI/FarmPlan/FarmPlanHUD.FarmPlanHUD_C"))
        (UserInterface|Viewport|AddtoViewport _returnvalue 0)
        (Variables|/Script/Engine.PlayerController|SetbShowMouseCursor (Game|GetPlayerController 0) true)
        (Variables|Default|SetIsShowFarmPlan true)))))

(fn ConstructionScript
  (bind _numberofground_x (Variables|Default|GetNumberOfGround_X))
  (bind _numberofground_y (Variables|Default|GetNumberOfGround_Y))
  (bind _groundsize (Variables|Default|GetGroundSize))
  (bind _groundsize_2 (Variables|Default|GetGroundSize))
  (for _index (range 1 _numberofground_x)
    (for _index_2 (range 1 _numberofground_y)
      (AddComponent|AddStaticMeshComponent false (Math|Transform|MakeTransform (+ "-50.000000,-50.000000, 0" (Math|Vector|MakeVector (- (* _index _groundsize) (/ (* _numberofground_x _groundsize_2) 2.0)) (- (* _index_2 _groundsize) (/ (* _numberofground_y _groundsize_2) 2.0)) 0.0)))))))